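; Security boss that fights with a health bar widget and opens the level door on death.
; After a start-up delay, Tick plays an awake sound and enters stage one.
; When the invincibility timer expires, it randomly toggles boss cell damage on then immediately off, spawns turrets or a bullet, or does nothing.
; TakeDamage triggers death at zero health, or stage two at half health, which Tick leaves unhandled.
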(event EventBeginPlay
  (Variables|Default|SetCurHealth (Variables|Default|GetMaxHealth))
  (bind _returnvalue (UserInterface|CreateWidget "/Game/UI/UI_BossStats.UI_BossStats_C"))
  (bind _output_get (Variables|Default|SetBossHealthBar _returnvalue))
  (UserInterface|Viewport|AddtoViewport _output_get 0)
  (bind _outactors (Actor|GetAllActorsOfClass "/Game/Blueprints/BP_BossCell.BP_BossCell_C"))
  (Variables|Default|SetCells _outactors))

(event Collision|EventActorBeginOverlap
  (params (OtherActor :type Actor%20Object%20Reference)))

(event EventTick
  (params (DeltaSeconds :type Float%20%28single-precision%29))
  (bind _cells (Variables|Default|GetCells))
  (switch int (Variables|Default|GetStage)
    (:0
      (bind _output_get (Variables|Default|Setbasetimer (+ (Variables|Default|Getbasetimer) DeltaSeconds)))
      (if (>= _output_get (Variables|Default|GetStartUpTime))
        (Variables|Default|Setbasetimer 0.0)
        (Variables|Default|SetStage 1)
        (Variables|Default|SetisActive true)
        (Audio|PlaySound2D "/Game/SoundEffects/bossawake.bossawake" 1.0 1.0 0.0 0 0)))
    (:1
      (if (not (Variables|Default|GetcanTakeDamage))
        (bind _output_get_2 (Variables|Default|SetinvinFrametimer (+ DeltaSeconds (Variables|Default|GetinvinFrametimer))))
        (if (>= _output_get_2 (Variables|Default|GetinvinFrameCooldown))
          (Variables|Default|SetinvinFrametimer 0.0)
          (Variables|Default|SetcanTakeDamage true)
          (switch int (Math|Random|RandomIntegerinRange 0 3)
            (:0
              (for _array_element _cells
                (Variables|/Game/Blueprints/BP_BossCell.BP_BossCell_C|SetCanHurtPlayer _array_element true))
              (for _array_element_2 _cells
                (Variables|/Game/Blueprints/BP_BossCell.BP_BossCell_C|SetCanHurtPlayer _array_element_2 false)))
            (:1
              (bind _array_element_3 (Utilities|Array|ForEachLoopwithBreak (Variables|Default|GetspawnLocals))
                (:LoopBody
                  (Game|SpawnActorfromClass "/Game/Blueprints/DefenseTurret.DefenseTurret_C" _array_element_3 "Undefined" "MultiplyWithRoot" 0 0))))
            (:2
              (Game|SpawnActorfromClass "/Game/Blueprints/TurretBullet.TurretBullet_C" (Transformation|GetActorTransform) "AlwaysSpawn" "MultiplyWithRoot" 0 0))))))))

(fn ConstructionScript)

(fn BossDeath
  (Audio|PlaySound2D "/Game/SoundEffects/bossdeath.bossdeath" 1.0 1.0 0.0 0 0)
  (Widget|RemovefromParent (Variables|Default|GetBossHealthBar))
  (bind _returnvalue (Actor|GetActorOfClass "/Game/Blueprints/LevelDoor.LevelDoor_C"))
  (Default|OpenDoor _returnvalue))

(fn TakeDamage
  (params (Amount :type Float%20%28double-precision%29))
  (bind _output_get (Variables|Default|SetCurHealth (- (Variables|Default|GetCurHealth) Amount)))
  (Audio|PlaySound2D 0 1.0 1.0 0.0 0 0)
  (if (<= _output_get 0.0)
    (CallFunction|BossDeath)
    (elif (<= (Variables|Default|GetCurHealth) (/ (Variables|Default|GetMaxHealth) 2.0))
      (Audio|PlaySound2D "/Game/SoundEffects/bossstageprogress.bossstageprogress" 1.0 1.0 0.0 0 0)
      (Variables|Default|SetStage 2))))