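; BP_Bullet is a projectile that deals the player's weapon damage to enemies and bosses.
; On spawn it offsets its yaw and schedules its destruction using the player's BulletLifetime.
; Tick moves it along the Arrow's forward vector by a fixed, frame-rate-dependent step without sweeping.
; Overlaps route BasicEnemy and BP_BossCell hits through the player's DealDamage without destroying the bullet, while TrainingDummy hits only destroy it after a brief delay.
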(event EventBeginPlay
  (bind _defaultsceneroot (Variables|Default|GetDefaultSceneRoot))
  (bind _returnvalue (Transformation|GetWorldRotation _defaultsceneroot))
  (Transformation|SetActorRotation (Math|Rotator|MakeRotator (.roll _returnvalue) (.pitch _returnvalue) (- (.yaw _returnvalue) 9e+01)))
  (bind _asbp_player (Utilities|Casting|CastToBP_Player (Game|GetPlayerCharacter 0)))
  (Utilities|FlowControl|Delay (Variables|/Game/Blueprints/BP_Player.BP_Player_C|GetBulletLifetime _asbp_player))
  (Actor|DestroyActor))

(event Collision|EventActorBeginOverlap
  (params (OtherActor :type Actor%20Object%20Reference))
  (Utilities|Casting|CastToTrainingDummy OtherActor
    (:then
      (Utilities|FlowControl|Delay 0.01)
      (Actor|DestroyActor))
    (:CastFailed
      (bind _asbasic_enemy (Utilities|Casting|CastToBasicEnemy OtherActor)
        (:then
          (bind _asbp_player (Utilities|Casting|CastToBP_Player (Game|GetPlayerCharacter 0)))
          (Default|DealDamage _asbp_player (Variables|/Game/Blueprints/BP_Player.BP_Player_C|GetWeaponDamage _asbp_player) _asbasic_enemy))
        (:CastFailed
          (bind _asbp_boss_cell (Utilities|Casting|CastToBP_BossCell OtherActor))
          (bind _asbp_player_2 (Utilities|Casting|CastToBP_Player (Game|GetPlayerCharacter 0)))
          (Default|DealDamage _asbp_player_2 (Variables|/Game/Blueprints/BP_Player.BP_Player_C|GetWeaponDamage _asbp_player_2) _asbp_boss_cell))))))

(event EventTick
  (params (DeltaSeconds :type Float%20%28single-precision%29))
  (bind _defaultsceneroot (Variables|Default|GetDefaultSceneRoot))
  (Transformation|SetWorldLocation _defaultsceneroot (+ (Transformation|GetWorldLocation _defaultsceneroot) (* (Math|Vector|GetForwardVector (Variables|Default|GetArrow)) 3e+01)) false false))

(fn ConstructionScript)