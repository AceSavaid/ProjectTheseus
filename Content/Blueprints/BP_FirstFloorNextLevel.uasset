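; Level-exit trigger for the first floor that sends BP_Player on to a random level from the game instance's FirstLevels list.
; On overlap it deactivates player movement and uses timelines to fade all point and directional lights toward zero intensity.
; From the directional-light fade update, after a delay, it increments CompletedLevels, flags the current level in WasPlayed1, rerolls to seek an unplayed index and calls TransitionToLevel.
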(event EventBeginPlay)

(event Collision|EventActorBeginOverlap
  (params (OtherActor :type Actor%20Object%20Reference))
  (bind _asbp_player (Utilities|Casting|CastToBP_Player OtherActor))
  (Components|Activation|SetActive (Variables|/Script/Engine.Character|GetCharacterMovement _asbp_player) false false)
  (bind _outactors (Actor|GetAllActorsOfClass "/Script/Engine.DirectionalLight"))
  (bind _outactors_2 (Actor|GetAllActorsOfClass "/Script/Engine.PointLight"))
  (Utilities|FlowControl|Sequence
    (:then_0
      (for _array_element _outactors_2
        (bind _newtrack_0 (Timeline|Timeline Play)
          (:Update
            (Rendering|Components|Light|SetIntensity (Variables|/Script/Engine.PointLight|GetPointLightComponent _array_element) (Math|Float|Lerp (Variables|/Script/Engine.LightComponentBase|GetIntensity (Variables|/Script/Engine.PointLight|GetPointLightComponent _array_element)) 0.0 _newtrack_0))))))
    (:then_1
      (for _array_element_2 _outactors
        (bind _newtrack_0_2 (Timeline|Timeline_0 Play)
          (:Update
            (Rendering|Components|Light|SetIntensity (Variables|/Script/Engine.Light|GetLightComponent _array_element_2) (Math|Float|Lerp (Variables|/Script/Engine.LightComponentBase|GetIntensity (Variables|/Script/Engine.Light|GetLightComponent _array_element_2)) 0.0 _newtrack_0_2))
            (Utilities|FlowControl|Delay 1.0)
            (Math|Integer|IncrementInt (Variables|/Game/Blueprints/BP_Player.BP_Player_C|GetCompletedLevels _asbp_player)
              (:%20%20
                (bind _result (Math|Integer|DecrementInt (Utilities|Array|Length (Variables|/Game/Blueprints/Persistence/GI_Persistent.GI_Persistent_C|GetFirst%20Levels (Default|GetGameInstance _asbp_player))))
                  (:%20%20
                    (Utilities|Array|SetArrayElem (Variables|/Game/Blueprints/Persistence/GI_Persistent.GI_Persistent_C|GetWasPlayed1 (Default|GetGameInstance _asbp_player)) (Variables|/Game/Blueprints/Persistence/GI_Persistent.GI_Persistent_C|GetCurrentLevel (Default|GetGameInstance _asbp_player)) true)
                    (if (Utilities|Array|Get(acopy) (Variables|/Game/Blueprints/Persistence/GI_Persistent.GI_Persistent_C|GetWasPlayed1 (Default|GetGameInstance _asbp_player)) (Math|Random|RandomIntegerinRange 0 _result))
                      (while (not (Utilities|Array|Get(acopy) (Variables|/Game/Blueprints/Persistence/GI_Persistent.GI_Persistent_C|GetWasPlayed1 (Default|GetGameInstance _asbp_player)) (Math|Random|RandomIntegerinRange 0 _result))) :!label _label
                        (bind _output_get (Variables|Default|SetRolledNumber (Math|Random|RandomIntegerinRange 0 _result)))
                        (if (== _output_get (Math|Random|RandomIntegerinRange 0 (Utilities|Array|Length (Variables|/Game/Blueprints/Persistence/GI_Persistent.GI_Persistent_C|GetFirst%20Levels (Default|GetGameInstance _asbp_player)))))
                          (Variables|Default|SetRolledNumber (Math|Random|RandomIntegerinRange 0 (Utilities|Array|Length (Variables|/Game/Blueprints/Persistence/GI_Persistent.GI_Persistent_C|GetFirst%20Levels (Default|GetGameInstance _asbp_player)))))
                          (goto _label)
                          (elif (Utilities|Array|Get(acopy) (Variables|/Game/Blueprints/Persistence/GI_Persistent.GI_Persistent_C|GetWasPlayed1 (Default|GetGameInstance _asbp_player)) (Variables|Default|GetRolledNumber))
                            (goto _label)
                            (else
                              (Default|TransitiontoLevel (Default|GetGameInstance _asbp_player) (Utilities|Array|Get(acopy) (Variables|/Game/Blueprints/Persistence/GI_Persistent.GI_Persistent_C|GetFirst%20Levels (Default|GetGameInstance _asbp_player)) (Variables|Default|GetRolledNumber)) _asbp_player (Variables|Default|GetRolledNumber))))))
                      (Default|TransitiontoLevel (Default|GetGameInstance _asbp_player) (Utilities|Array|Get(acopy) (Variables|/Game/Blueprints/Persistence/GI_Persistent.GI_Persistent_C|GetFirst%20Levels (Default|GetGameInstance _asbp_player)) (Variables|Default|GetRolledNumber)) _asbp_player (Variables|Default|GetRolledNumber))
                      (else
                        (Default|TransitiontoLevel (Default|GetGameInstance _asbp_player) (Utilities|Array|Get(acopy) (Variables|/Game/Blueprints/Persistence/GI_Persistent.GI_Persistent_C|GetFirst%20Levels (Default|GetGameInstance _asbp_player)) (Math|Random|RandomIntegerinRange 0 _result)) _asbp_player (Math|Random|RandomIntegerinRange 0 _result))))))))))))))

(event EventTick
  (params (DeltaSeconds :type Float%20%28single-precision%29)))

(fn ConstructionScript)