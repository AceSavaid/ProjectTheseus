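; Player character for an isometric action game with cursor-facing aim, pause and upgrade-station menus, and swappable body parts.
; Equipped legs, arms, chest and head select dash or sprint, melee or ranged attack, health/speed frame and healing, and are restored from GI_Persistent on level transitions.
; DealDamage applies upgrade bonuses and handles enemy deaths, drops and opening level doors at the kill goal.
; Fatal contact damage loads the death screen.
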(event OnComponentBeginOverlap(CapsuleComponent)
  (params (OverlappedComponent :type Primitive%20Component%20Object%20Reference) (OtherActor :type Actor%20Object%20Reference) (OtherComp :type Primitive%20Component%20Object%20Reference) (OtherBodyIndex :type Integer) (bFromSweep :type Boolean) (SweepResult :type Hit%20Result%20Structure%20%28by%20ref%29))
  (bind _asbasic_enemy (Utilities|Casting|CastToBasicEnemy OtherActor))
  (bind _diedfromdamage (CallFunction|TakeDamage (Variables|/Game/Blueprints/Enemies/BasicEnemy.BasicEnemy_C|GetEnemyDamage _asbasic_enemy)))
  (if _diedfromdamage
    (Game|OpenLevel(byName) "DeathScreen")))

(event Custom|OnComponentBeginOverlap
  (params (OverlappedComponent :type Primitive%20Component%20Object%20Reference) (OtherActor :type Actor%20Object%20Reference) (OtherComp :type Primitive%20Component%20Object%20Reference) (OtherBodyIndex :type Integer) (bFromSweep :type Boolean) (SweepResult :type Hit%20Result%20Structure%20%28by%20ref%29))
  ;[1 1 1] Attacking (Melee)
  (Utilities|Casting|CastToTrainingDummy OtherActor
    (:then
      (if (not (Variables|Default|GetHit%20cooldown%20active))
        (Variables|Default|SetHit%20cooldown%20active true)
        (Utilities|FlowControl|Delay (Variables|Default|GetSword%20hitbox%20cooldown))
        (Variables|Default|SetHit%20cooldown%20active false)))
    (:CastFailed
      (bind _asbasic_enemy (Utilities|Casting|CastToBasicEnemy OtherActor)
        (:then
          (if (not (Variables|Default|GetHit%20cooldown%20active))
            (CallFunction|DealDamage (Variables|Default|GetWeaponDamage) _asbasic_enemy)
            (Variables|Default|SetHit%20cooldown%20active true :!label _label)
            (Utilities|FlowControl|Delay (Variables|Default|GetSword%20hitbox%20cooldown))
            (Variables|Default|SetHit%20cooldown%20active false)))
        (:CastFailed
          (bind _asbp_boss_cell (Utilities|Casting|CastToBP_BossCell OtherActor))
          (if (not (Variables|Default|GetHit%20cooldown%20active))
            (CallFunction|DealDamage (Variables|Default|GetWeaponDamage) _asbp_boss_cell)
            (goto _label)))))))

(event Custom|InvertPause
  (Variables|Default|SetIsPaused (not (Variables|Default|GetIsPaused))))

(event Input|EnhancedActionEvents|EnhancedInputActionIA_Move
  (params (ActionValue :type Vector%202D%20Structure) (ElapsedSeconds :type Float%20%28double-precision%29) (TriggeredSeconds :type Float%20%28double-precision%29) (InputAction :type Input%20Action%20Object%20Reference :default "/Game/Input/IA_Move.IA_Move"))
  (bind (_x _y) (Math|Vector2D|BreakVector2D ActionValue))
  ;[1 1 1] WASD movement
  (if (not (Variables|Default|GetDash%20cooldown))
    (Pawn|Input|AddMovementInput (+ (Transformation|GetActorRightVector) (Variables|Default|GetIsometric%20Correction%20%28X%29)) _x false)
    (Pawn|Input|AddMovementInput (+ (Transformation|GetActorForwardVector) (Variables|Default|GetIsometric%20Correction%20%28Y%29)) _y false)))

(event Input|EnhancedActionEvents|EnhancedInputActionIA_Attack
  (params (ActionValue :type Boolean) (ElapsedSeconds :type Float%20%28double-precision%29) (TriggeredSeconds :type Float%20%28double-precision%29) (InputAction :type Input%20Action%20Object%20Reference :default "/Game/Input/IA_Attack.IA_Attack"))
  (bind _hitbox (Variables|Default|GetHitbox))
  (bind _arms (Variables|Default|GetArms))
  (bind _arrow1 (Variables|Default|GetArrow1))
  (bind _equips (Variables|Default|GetEquips))
  (bind _output (Utilities|Array|Get(acopy) _equips _arms))
  ;[1 1 1] Attacking (Melee)
  (if (Utilities|Enum|Equal(Enum) _output "melee")
    (Collision|SetCollisionEnabled _hitbox "QueryAndPhysics")
    (Audio|SpawnSound2D "/Game/SoundEffects/meleeattack.meleeattack" 1.0 1.0 0.0 0)
    (Development|SetHiddeninGame (Variables|Default|GetParent) false true)
    (Utilities|FlowControl|Delay (Variables|Default|GetAttack%20Speed))
    (Collision|SetCollisionEnabled _hitbox "NoCollision")
    (Development|SetHiddeninGame (Variables|Default|GetParent) true true)
    (elif (Utilities|Enum|Equal(Enum) _output "ranged")
      (if (not (Variables|Default|GetHit%20cooldown%20active))
        (Variables|Default|SetHit%20cooldown%20active true)
        (Audio|PlaySound2D "/Game/SoundEffects/laser_prototyple2.laser_prototyple2" 1.0 1.0 0.0 0 0)
        (Game|SpawnActorfromClass "/Game/Blueprints/BP_Bullet.BP_Bullet_C" (Math|Transform|MakeTransform (+ (Transformation|GetWorldLocation _arrow1) (* (Math|Vector|GetForwardVector _arrow1) 5.0)) (Transformation|GetWorldRotation _arrow1) "1.000000,1.000000,1.000000") "AdjustIfPossibleButAlwaysSpawn" "MultiplyWithRoot" 0 0)
        (Utilities|FlowControl|Delay (Variables|Default|GetSword%20hitbox%20cooldown))
        (Variables|Default|SetHit%20cooldown%20active false)))))

(event Input|EnhancedActionEvents|EnhancedInputActionIA_ClassAction
  (params (ActionValue :type Boolean) (ElapsedSeconds :type Float%20%28double-precision%29) (TriggeredSeconds :type Float%20%28double-precision%29) (InputAction :type Input%20Action%20Object%20Reference :default "/Game/Input/IA_ClassAction.IA_ClassAction"))
  (bind _equips (Variables|Default|GetEquips))
  (bind _legs (Variables|Default|GetLegs))
  (bind _charactermovement (Variables|Character|GetCharacterMovement))
  (bind _output (Utilities|Array|Get(acopy) _equips _legs))
  (bind _returnvalue (Utilities|Enum|Equal(Enum) _output "sprint"))
  (:Triggered
    (if (Utilities|Enum|Equal(Enum) _output "dash")
      (if (not (Variables|Default|GetDash%20cooldown))
        (Variables|Default|SetY%20movement%20scale (.Y (Math|Vector2D|BreakVector2D (stale Input|EnhancedActionEvents|EnhancedInputActionIA_Move ActionValue))))
        (Variables|Default|SetX%20movement%20scale (.X (Math|Vector2D|BreakVector2D (stale Input|EnhancedActionEvents|EnhancedInputActionIA_Move ActionValue))))
        (Variables|Default|SetDash%20cooldown true)
        (Variables|/Script/Engine.CharacterMovementComponent|SetMaxWalkSpeed (Variables|Character|GetCharacterMovement) (Variables|Default|GetDash%20speed))
        (Utilities|FlowControl|Sequence
          (:then_0
            (Timeline|Timeline Play
              (:Update
                (Pawn|Input|AddMovementInput (+ (Transformation|GetActorRightVector) (Variables|Default|GetIsometric%20Correction%20%28X%29)) (Variables|Default|GetX%20movement%20scale) false)
                (Pawn|Input|AddMovementInput (+ (Transformation|GetActorForwardVector) (Variables|Default|GetIsometric%20Correction%20%28Y%29)) (Variables|Default|GetY%20movement%20scale) false))
              (:Finished
                (Variables|Default|SetDash%20cooldown false :!label _label)
                (Variables|/Script/Engine.CharacterMovementComponent|SetMaxWalkSpeed (Variables|Character|GetCharacterMovement) (Variables|Default|GetcurrentWalkSpeed))
                (Timeline|Timeline Stop))))
          (:then_1
            (Utilities|FlowControl|Delay (Variables|Default|GetDash%20Duration))
            (goto _label))))
      (elif _returnvalue
        (Variables|/Script/Engine.CharacterMovementComponent|SetMaxWalkSpeed _charactermovement (Variables|Default|GetcurrentWalkSpeed)))))
  (:Ongoing
    (if _returnvalue
      (Variables|/Script/Engine.CharacterMovementComponent|SetMaxWalkSpeed _charactermovement (* (Variables|Default|GetcurrentWalkSpeed) 1.666667)))))

(event Input|EnhancedActionEvents|EnhancedInputActionIA_Interact
  (params (ActionValue :type Boolean) (ElapsedSeconds :type Float%20%28double-precision%29) (TriggeredSeconds :type Float%20%28double-precision%29) (InputAction :type Input%20Action%20Object%20Reference :default "/Game/Input/IA_Interact.IA_Interact"))
  ;[1 1 1] Upgrade Station Interaction
  (if (Variables|Default|GetInStation)
    (if (Utilities|IsValid (Variables|Default|GetUpgrade%20Station%20UI))
      (UserInterface|Viewport|AddtoViewport (Variables|Default|GetUpgrade%20Station%20UI) 0)
      (Utilities|Time|SetGlobalTimeDilation 0.0)
      (else
        (bind _returnvalue (UserInterface|CreateWidget "/Game/UI/UI_UpgradeStation.UI_UpgradeStation_C" (Game|GetPlayerController 0)))
        (bind _output_get (Variables|Default|SetUpgrade%20Station%20UI _returnvalue))
        (UserInterface|Viewport|AddtoViewport _output_get 0)
        (Utilities|Time|SetGlobalTimeDilation 0.0)))))

(event Input|EnhancedActionEvents|EnhancedInputActionIA_Pause
  (params (ActionValue :type Boolean) (ElapsedSeconds :type Float%20%28double-precision%29) (TriggeredSeconds :type Float%20%28double-precision%29) (InputAction :type Input%20Action%20Object%20Reference :default "/Game/Input/IA_Pause.IA_Pause"))
  ;[1 1 1] Pause Menu Function - (Alanns did this) Opens the Pause menu widget and freezes time
  ; Checks to see if the game is already paused.
  ; If it is not paused, it pauses the game and opens the pause menu.  If it is pause it closes the pause menu and resumes the game.
  (if (Variables|Default|GetIsPaused)
    (CallFunction|InvertPause)
    (bind _returnvalue (UserInterface|CreateWidget "/Game/UI/UI_PauseMenu.UI_PauseMenu_C"))
    (bind _output_get (Variables|Default|SetPauseMenuUI _returnvalue))
    (UserInterface|Viewport|AddtoViewport _output_get 0)
    (Utilities|Time|SetGlobalTimeDilation 0.0)
    (else
      (CallFunction|InvertPause)
      (Widget|RemovefromParent (Variables|Default|GetPauseMenuUI))
      (Utilities|Time|SetGlobalTimeDilation 1.0))))

(event EventBeginPlay
  ;[1 1 1] Linking input to player
  (bind _asplayer_controller (Utilities|Casting|CastToPlayerController (Pawn|GetController)))
  (Utilities|IsValid (PlayerController|LocalPlayerSubsystems|GetEnhancedInputLocalPlayerSubsystem _asplayer_controller)
    (:Is%20Valid
      (Input|AddMappingContext (PlayerController|LocalPlayerSubsystems|GetEnhancedInputLocalPlayerSubsystem _asplayer_controller) "/Game/Input/IMC.IMC" 0 "(bIgnoreAllPressedKeysUntilRelease=True,bForceImmediately=False,bNotifyUserSettings=False)")
      (Variables|/Script/Engine.PlayerController|SetbShowMouseCursor (Game|GetPlayerController 0) true)
      ;[1 1 1] Attacking (Melee)
      (Collision|AssignOnComponentBeginOverlap (Variables|Default|GetHitbox) (delegate Custom|OnComponentBeginOverlap))
      (if (Variables|/Game/Blueprints/Persistence/GI_Persistent.GI_Persistent_C|GetShouldLoadTransition (CallFunction|GetGameInstance))
        (CallFunction|LoadPlayerState))
      (bind _outactors (Actor|GetAllActorsOfClass (Variables|Default|GetBasicEnemy%20Ref)))
      (Variables|Default|SetCurrentEnemies (Utilities|Array|Length _outactors))
      (Timeline|Healing_Time Play
        (:Update
          (Utilities|FlowControl|Delay (Variables|Default|GetHealTime))
          (if (Utilities|Enum|Equal(Enum) (Utilities|Array|Get(acopy) (Variables|Default|GetEquips) (Variables|Default|GetHead)) "truesight")
            (if (< (Variables|Default|GetcurrentHealth) (Variables|Default|GetMaxHealth))
              (Math|Float|IncrementFloat (Variables|Default|GetcurrentHealth)))))))))

(event EventTick
  (params (DeltaSeconds :type Float%20%28single-precision%29))
  (bind _returnvalue (Transformation|GetActorRotation))
  ;[1 1 1] Player Look Rotation
  (Transformation|SetWorldRotation (Variables|Default|GetCylinder) (Math|Rotator|MakeRotator (.roll _returnvalue) (.pitch _returnvalue) (.yaw (Math|Rotator|FindLookatRotation (Transformation|GetActorLocation) (.Location (Collision|BreakHitResult (.HitResult (Game|Player|GetHitResultUnderCursorbyChannel (Game|GetPlayerController 0) "TraceTypeQuery1" true))))))) false false))

(fn ConstructionScript
  (Collision|SetCollisionEnabled (Variables|Default|GetHitbox) "NoCollision")
  (Development|SetHiddeninGame (Variables|Default|GetParent) true true))

(fn TakeDamage
  (params (Damage%20Taken :type Float%20%28double-precision%29))
  (bind _output_get (Variables|Default|SetcurrentHealth (- (Variables|Default|GetcurrentHealth) Damage%20Taken)))
  (Audio|SpawnSoundatLocation "/Game/SoundEffects/playerhurt.playerhurt" (Transformation|GetActorLocation) "0, 0, 0" 1.0 1.0 0.0 0 0)
  (if (<= _output_get 0.0)
    (LocalVariables|SetNewLocalVar true)
    (else
      (LocalVariables|SetNewLocalVar false)))
  (return (LocalVariables|GetNewLocalVar)))

(fn DealDamage
  (params (WeaponDamage :type Float%20%28double-precision%29) (HitTarget :type Actor%20Object%20Reference))
  (bind _powerups (Variables|Default|GetPowerups))
  (bind _asbasic_enemy (Utilities|Casting|CastToBasicEnemy HitTarget)
    (:then
      ;[1 1 1] Bloodlust heals 2% on attacks. Stacks.
      (if (Variables|Default|GethasBloodLust)
        (Variables|Default|SetcurrentHealth (+ (Variables|Default|GetcurrentHealth) (* (Variables|Default|GetMaxHealth) (Variables|Default|GetBloodLustValue))))
        ;[1 1 1] Holdstill deals 5 extra damage if not moving. Stacks.
        (if (Variables|Default|GetHas%20HoldStill)
          (if (and (== (Variables|Default|GetX%20movement%20scale) 0.0) (== (Variables|Default|GetY%20movement%20scale) 0.0))
            (Variables|/Game/Blueprints/Enemies/BasicEnemy.BasicEnemy_C|SetEnemyHealth _asbasic_enemy (+ (- (Variables|/Game/Blueprints/Enemies/BasicEnemy.BasicEnemy_C|GetEnemyHealth _asbasic_enemy) (+ WeaponDamage (Variables|Default|GetHoldStillValue))) (Variables|/Game/Blueprints/Enemies/BasicEnemy.BasicEnemy_C|GetEnemyDefense _asbasic_enemy)))
            (if (<= (stale _output_get) 0.0) :!label _label
              (bind _asslime_enemy_2 (Utilities|Casting|CastToSlimeEnemy2 _asbasic_enemy)
                (:then
                  (bind _returnvalue (Game|SpawnActorfromClass "/Game/Blueprints/Enemies/SlimeResidue.SlimeResidue_C" (Transformation|GetActorTransform _asslime_enemy_2) "AdjustIfPossibleButAlwaysSpawn" "MultiplyWithRoot" 0 0))
                  (Variables|/Game/Blueprints/Enemies/SlimeResidue.SlimeResidue_C|SetSlimeDamage _returnvalue (Variables|/Game/Blueprints/Enemies/SlimeEnemy2.SlimeEnemy2_C|GetSlimeDamage _asslime_enemy_2)))
                (:CastFailed
                  _))
              (if (== (Math|Integer|%(Integer) (Math|Random|RandomIntegerinRange 1 5) 5) 0)
                (Game|SpawnActorfromClass (Utilities|Array|Get(acopy) _powerups (Math|Random|RandomIntegerinRange 0 (Utilities|Array|Length _powerups))) (Transformation|GetActorTransform _asbasic_enemy) "AdjustIfPossibleButAlwaysSpawn" "MultiplyWithRoot" 0 0))
              (Actor|DestroyActor _asbasic_enemy)
              (Math|Integer|DecrementInt (Variables|Default|GetCurrentEnemies)
                (:%20%20
                  (Math|Integer|IncrementInt (Variables|Default|GetKills)
                    (:%20%20
                      (if (>= (Variables|Default|GetKills) (Variables|Default|GetKillGoal))
                        (bind _outactors (Actor|GetAllActorsOfClass "/Game/Blueprints/LevelDoor.LevelDoor_C"))
                        (for _array_element _outactors
                          (Default|OpenDoor _array_element)))))))))
          (else
            (bind _output_get (Variables|/Game/Blueprints/Enemies/BasicEnemy.BasicEnemy_C|SetEnemyHealth _asbasic_enemy (+ (- (Variables|/Game/Blueprints/Enemies/BasicEnemy.BasicEnemy_C|GetEnemyHealth _asbasic_enemy) WeaponDamage) (Variables|/Game/Blueprints/Enemies/BasicEnemy.BasicEnemy_C|GetEnemyDefense _asbasic_enemy)) :!label _label_2))
            (goto _label)))
        (else
          (goto _label_2))))
    (:CastFailed
      (bind _asbp_boss_cell (Utilities|Casting|CastToBP_BossCell HitTarget))
      (Default|TakeDamage _asbp_boss_cell WeaponDamage))))

(fn GetGameInstance
  (bind _asgi_persistent (Utilities|Casting|CastToGI_Persistent (Game|GetGameInstance)))
  (return _asgi_persistent))

(fn LoadPlayerState
  (bind _out (CallFunction|GetGameInstance))
  (bind _output_get (Variables|Default|SetEquips (Variables|/Game/Blueprints/Persistence/GI_Persistent.GI_Persistent_C|GetEquips _out)))
  (Utilities|FlowControl|Sequence
    (:then_0
      (CallFunction|LoadLegs (Utilities|Array|Get(acopy) _output_get (Variables|Default|GetLegs))))
    (:then_1
      (CallFunction|LoadArms (Utilities|Array|Get(acopy) _output_get (Variables|Default|GetArms))))
    (:then_2
      (CallFunction|LoadChest (Utilities|Array|Get(acopy) _output_get (Variables|Default|GetChest))))
    (:then_3
      (CallFunction|LoadHead (Utilities|Array|Get(acopy) _output_get (Variables|Default|GetHead))))
    (:then_4
      (Variables|Default|SetcurrentWalkSpeed (Variables|/Game/Blueprints/Persistence/GI_Persistent.GI_Persistent_C|GetSpeed _out))
      (Variables|Default|SetbaseHealth (Variables|/Game/Blueprints/Persistence/GI_Persistent.GI_Persistent_C|GetHealth _out))
      (Variables|Default|SetWeaponDamage (Variables|/Game/Blueprints/Persistence/GI_Persistent.GI_Persistent_C|GetDamage _out))
      (Variables|Default|SetcurrentHealth (Variables|/Game/Blueprints/Persistence/GI_Persistent.GI_Persistent_C|GetCurrentHealth _out)))
    (:then_5
      (Variables|/Game/Blueprints/Persistence/GI_Persistent.GI_Persistent_C|SetShouldLoadTransition _out false))
    (:then_6
      (Variables|Default|SetCompletedLevels (Variables|/Game/Blueprints/Persistence/GI_Persistent.GI_Persistent_C|GetCompletedLevels _out)))))

(fn LoadLegs
  (params (Legs :type String))
  (bind _asbp_player (Utilities|Casting|CastToBP_Player (Game|GetPlayerCharacter 0)))
  (Utilities|Array|SetArrayElem (Variables|BP_Player_C|GetEquips _asbp_player) (Variables|BP_Player_C|GetLegs _asbp_player) Legs)
  (switch string Legs
    (:dash
      (Components|StaticMesh|SetStaticMesh (Variables|BP_Player_C|GetRobo%20Rabbit%201%20Legs _asbp_player) "/Game/StuffThatCouldBeScrap/RabbitLegs.RabbitLegs"))
    (:sprint
      (Components|StaticMesh|SetStaticMesh (Variables|BP_Player_C|GetRobo%20Rabbit%201%20Legs _asbp_player) "/Game/Models/Characters/DeerLegs.DeerLegs"))))

(fn LoadArms
  (params (Arms :type String))
  (bind _asbp_player (Utilities|Casting|CastToBP_Player (Game|GetPlayerCharacter 0)))
  (Utilities|Array|SetArrayElem (Variables|BP_Player_C|GetEquips _asbp_player) (Variables|BP_Player_C|GetArms _asbp_player) Arms)
  (switch string Arms
    (:melee
      (Components|StaticMesh|SetStaticMesh (Variables|BP_Player_C|GetWWJD_Arms__Rabbit__-_MODIFIED _asbp_player) "/Game/Models/Characters/DeerArm.DeerArm"))
    (:ranged
      (Components|StaticMesh|SetStaticMesh (Variables|BP_Player_C|GetWWJD_Arms__Rabbit__-_MODIFIED _asbp_player) "/Game/StuffThatCouldBeScrap/RabbitArms.RabbitArms"))))

(fn LoadChest
  (params (Chest :type String))
  (bind _asbp_player (Utilities|Casting|CastToBP_Player (Game|GetPlayerCharacter 0)))
  (Utilities|Array|SetArrayElem (Variables|BP_Player_C|GetEquips _asbp_player) (Variables|BP_Player_C|GetChest _asbp_player) Chest)
  (Variables|Default|Setmax%20health%20before%20it%20was%20changed (Variables|BP_Player_C|GetMaxHealth _asbp_player))
  (if (Utilities|Enum|Equal(Enum) Chest "heavy frame")
    (bind _output_get (Variables|/Script/Engine.CharacterMovementComponent|SetMaxWalkSpeed (Variables|/Script/Engine.Character|GetCharacterMovement _asbp_player) (* (Variables|BP_Player_C|GetbaseWalkSpeed _asbp_player) 0.8)))
    (Variables|BP_Player_C|SetcurrentWalkSpeed _asbp_player _output_get)
    (Variables|BP_Player_C|SetMaxHealth _asbp_player (* (Variables|BP_Player_C|GetbaseHealth _asbp_player) 1.2))
    (else
      (bind _output_get_2 (Variables|/Script/Engine.CharacterMovementComponent|SetMaxWalkSpeed (Variables|/Script/Engine.Character|GetCharacterMovement _asbp_player) (* (Variables|BP_Player_C|GetbaseWalkSpeed _asbp_player) 1.2)))
      (Variables|BP_Player_C|SetcurrentWalkSpeed _asbp_player _output_get_2)
      (Variables|BP_Player_C|SetMaxHealth _asbp_player (* (Variables|BP_Player_C|GetbaseHealth _asbp_player) 0.8))))
  (Variables|BP_Player_C|SetcurrentHealth _asbp_player (* (/ (Variables|BP_Player_C|GetcurrentHealth _asbp_player) (Variables|Default|Getmax%20health%20before%20it%20was%20changed)) (Variables|BP_Player_C|GetMaxHealth _asbp_player)))
  (switch string Chest
    (:heavy%20frame
      (Components|StaticMesh|SetStaticMesh (Variables|BP_Player_C|GetJonathan_Doe_Torso _asbp_player) "/Game/Models/Characters/DeerTorso.DeerTorso"))
    (:light%20frame
      (Components|StaticMesh|SetStaticMesh (Variables|BP_Player_C|GetJonathan_Doe_Torso _asbp_player) "/Game/StuffThatCouldBeScrap/RabbitTorso.RabbitTorso"))))

(fn LoadHead
  (params (Head :type String))
  (bind _asbp_player (Utilities|Casting|CastToBP_Player (Game|GetPlayerCharacter 0)))
  (Utilities|Array|SetArrayElem (Variables|BP_Player_C|GetEquips _asbp_player) (Variables|BP_Player_C|GetHead _asbp_player) Head)
  (switch string Head
    (:blindsight
      (Components|StaticMesh|SetStaticMesh (Variables|BP_Player_C|GetRoboRabbit_1__Head _asbp_player) "/Game/Models/Characters/DeerHead.DeerHead"))
    (:truesight
      (Components|StaticMesh|SetStaticMesh (Variables|BP_Player_C|GetRoboRabbit_1__Head _asbp_player) "/Game/StuffThatCouldBeScrap/RabbitHead.RabbitHead"))))

(fn AddUpgradetoList
  (params (UpgradeName :type String))
  (Utilities|Array|Add (Variables|Default|GetUpgradeList) UpgradeName))