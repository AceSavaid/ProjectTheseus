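; BP_BossCell is a damageable cell in the BP_BossSecurity fight that doubles as a turret and electric hazard.
; Flags drive Tick: ShootAtPlayer turns it toward the player and fires on a timer, while Turret spins the cylinder and fires along its arrow.
; CanHurtPlayer toggles electricity outside aiming mode and enables sphere-overlap damage.
; TakeDamage forwards damage to the boss and its own hit points, disabling further damage at zero.
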(event OnComponentBeginOverlap(Sphere)
  (params (OverlappedComponent :type Primitive%20Component%20Object%20Reference) (OtherActor :type Actor%20Object%20Reference) (OtherComp :type Primitive%20Component%20Object%20Reference) (OtherBodyIndex :type Integer) (bFromSweep :type Boolean) (SweepResult :type Hit%20Result%20Structure%20%28by%20ref%29))
  (if (Variables|Default|GetCanHurtPlayer)
    (bind _asbp_player (Utilities|Casting|CastToBP_Player OtherActor))
    (Default|TakeDamage _asbp_player 5.0)))

(event EventBeginPlay
  (Variables|Default|SetCurHitPoints (Variables|Default|GetMaxHitPoints))
  (bind _returnvalue (Actor|GetActorOfClass "/Game/Blueprints/Boses/Floor1/BP_BossSecurity.BP_BossSecurity_C"))
  (Variables|Default|SetBoss _returnvalue))

(event EventTick
  (params (DeltaSeconds :type Float%20%28single-precision%29))
  (bind _batteryelectricity (Variables|Default|GetBatteryElectricity))
  (bind _returnvalue (Components|Activation|IsActive _batteryelectricity))
  (if (Variables|Default|GetShootAtPlayer)
    (bind _returnvalue_2 (Actor|GetActorOfClass "/Game/Blueprints/BP_Player.BP_Player_C"))
    (Transformation|AddActorLocalRotation (Math|Rotator|FindRelativeLookatRotation (Transformation|GetActorTransform) (Transformation|GetActorLocation _returnvalue_2)) false false)
    (bind _output_get (Variables|Default|SetTshoottimer (+ DeltaSeconds (Variables|Default|GetTshoottimer))))
    (if (>= _output_get (Variables|Default|GetTshootTime))
      (Variables|Default|SetTshoottimer 0.0)
      (Audio|PlaySound2D "/Game/SoundEffects/turretshoot.turretshoot" 1.0 1.0 0.0 0 0)
      (Game|SpawnActorfromClass "/Game/Blueprints/TurretBullet.TurretBullet_C" (Transformation|GetWorldTransform (Variables|Default|GetArrow)) "AlwaysSpawn" "MultiplyWithRoot" 0 0))
    (else
      (if (Variables|Default|GetCanHurtPlayer)
        (if _returnvalue
          _
          (else
            (Components|Activation|Activate _batteryelectricity false)
            (Audio|PlaySound2D "/Game/SoundEffects/batteryElectrocute.batteryElectrocute" 1.0 1.0 0.0 0 0)))
        (elif _returnvalue
          (Components|Activation|Deactivate _batteryelectricity)))
      (if (Variables|Default|Getturret)
        (Transformation|AddLocalRotation (Variables|Default|GetCylinder) "0.000000,3.000000,0.000000" false false)
        (bind _output_get_2 (Variables|Default|SetTshoottimer (+ DeltaSeconds (Variables|Default|GetTshoottimer))))
        (if (>= _output_get_2 (Variables|Default|GetTshootTime))
          (Variables|Default|SetTshoottimer 0.0)
          (Audio|SpawnSoundatLocation "/Game/SoundEffects/turretshoot.turretshoot" (Transformation|GetActorLocation) "0, 0, 0" 1.0 1.0 0.0 0 0)
          (Game|SpawnActorfromClass "/Game/Blueprints/TurretBullet.TurretBullet_C" (Transformation|GetWorldTransform (Variables|Default|GetArrow)) "AlwaysSpawn" "MultiplyWithRoot" 0 0))))))

(fn ConstructionScript)

(fn TakeDamage
  (params (Amount :type Float%20%28double-precision%29))
  (if (Variables|Default|GetCanTakeDamage)
    (Audio|PlaySound2D 0 1.0 1.0 0.0 0 0)
    (Default|TakeDamage (Variables|Default|GetBoss) Amount)
    (bind _output_get (Variables|Default|SetCurHitPoints (- (Variables|Default|GetCurHitPoints) Amount)))
    (if (<= _output_get 0.0)
      (Variables|Default|SetCanTakeDamage false)
      (Audio|PlaySound2D 0 1.0 1.0 0.0 0 0))))