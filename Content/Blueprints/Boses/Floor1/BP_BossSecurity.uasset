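; Floor 1 security boss that fights through the level's BP_BossCell actors and shows a health bar widget.
; Tick waits out a startup timer, then periodically picks one of four random attacks by briefly toggling cell flags for electrocution, turret, both, or shooting at the player.
; TakeDamage enters a second stage at half health by setting a new attack interval, and at zero calls BossDeath, which removes the bar and opens the LevelDoor.
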(event EventBeginPlay
  (Variables|Default|SetCurHealth (Variables|Default|GetMaxHealth))
  (bind _returnvalue (UserInterface|CreateWidget "/Game/UI/UI_Boss1Stats.UI_Boss1Stats_C"))
  (bind _output_get (Variables|Default|SetBossHealthBar _returnvalue))
  (UserInterface|Viewport|AddtoViewport _output_get 0)
  (bind _outactors (Actor|GetAllActorsOfClass "/Game/Blueprints/Boses/Floor1/BP_BossCell.BP_BossCell_C"))
  (Variables|Default|SetCells _outactors))

(event Collision|EventActorBeginOverlap
  (params (OtherActor :type Actor%20Object%20Reference)))

(event EventTick
  (params (DeltaSeconds :type Float%20%28single-precision%29))
  (bind _cells (Variables|Default|GetCells))
  (bind _timebetweenattacks (Variables|Default|GettimeBetweenAttacks))
  (bind _cells_2 (Variables|Default|GetCells))
  (bind _cells_3 (Variables|Default|GetCells))
  (bind _cells_4 (Variables|Default|GetCells))
  (switch int (Variables|Default|GetStage)
    (:0
      (bind _output_get (Variables|Default|Setbasetimer (+ (Variables|Default|Getbasetimer) DeltaSeconds)))
      (if (>= _output_get (Variables|Default|GetStartUpTime))
        (Variables|Default|Setbasetimer 0.0)
        (Variables|Default|SetStage 1)
        (Variables|Default|SetisActive true)
        (Audio|PlaySound2D "/Game/SoundEffects/bossawake.bossawake" 1.0 1.0 0.0 0 0)
        (Variables|Default|SetcanAttack true)))
    (:1
      (if (Variables|Default|GetcanAttack) :!label _label
        (bind _output_get_2 (Variables|Default|SetAttackTimer (+ DeltaSeconds (Variables|Default|GetAttackTimer))))
        (if (>= _output_get_2 (Variables|Default|GetAttackTime))
          (Variables|Default|SetAttackTimer 0.0)
          (Variables|Default|SetattactTimeUp true)
          (if (Variables|Default|GetcanAttack)
            (switch int (Math|Random|RandomIntegerinRange 0 3)
              (:0
                ;[1 1 1] Battery Electrocution
                (Variables|Default|SetcanAttack false)
                (for _array_element _cells_3
                  (Variables|/Game/Blueprints/Boses/Floor1/BP_BossCell.BP_BossCell_C|SetCanHurtPlayer _array_element true))
                (Utilities|FlowControl|Delay 3.0)
                (for _array_element_2 _cells_3
                  (Variables|/Game/Blueprints/Boses/Floor1/BP_BossCell.BP_BossCell_C|SetCanHurtPlayer _array_element_2 false))
                (Utilities|FlowControl|Delay _timebetweenattacks)
                (Variables|Default|SetcanAttack true))
              (:1
                ;[1 1 1] Turrent
                (Variables|Default|SetcanAttack false)
                (for _array_element_3 _cells_2
                  (Variables|/Game/Blueprints/Boses/Floor1/BP_BossCell.BP_BossCell_C|Setturret _array_element_3 true))
                (Utilities|FlowControl|Delay 3.0)
                (for _array_element_4 _cells_2
                  (Variables|/Game/Blueprints/Boses/Floor1/BP_BossCell.BP_BossCell_C|Setturret _array_element_4 false))
                (Utilities|FlowControl|Delay _timebetweenattacks)
                (Variables|Default|SetcanAttack true))
              (:2
                ;[1 1 1] Electrocute and Shoot
                (Variables|Default|SetcanAttack false)
                (for _array_element_5 _cells
                  (Variables|/Game/Blueprints/Boses/Floor1/BP_BossCell.BP_BossCell_C|Setturret _array_element_5 true)
                  (Variables|/Game/Blueprints/Boses/Floor1/BP_BossCell.BP_BossCell_C|SetCanHurtPlayer _array_element_5 true))
                (Utilities|FlowControl|Delay 3.0)
                (for _array_element_6 _cells
                  (Variables|/Game/Blueprints/Boses/Floor1/BP_BossCell.BP_BossCell_C|Setturret _array_element_6 false)
                  (Variables|/Game/Blueprints/Boses/Floor1/BP_BossCell.BP_BossCell_C|SetCanHurtPlayer _array_element_6 false))
                (Utilities|FlowControl|Delay _timebetweenattacks)
                (Variables|Default|SetcanAttack true))
              (:3
                ;[1 1 1] Comment
                (Variables|Default|SetcanAttack false)
                (for _array_element_7 _cells_4
                  (Variables|/Game/Blueprints/Boses/Floor1/BP_BossCell.BP_BossCell_C|SetShootAtPlayer _array_element_7 true))
                (Utilities|FlowControl|Delay 3.0)
                (for _array_element_8 _cells_4
                  (Variables|/Game/Blueprints/Boses/Floor1/BP_BossCell.BP_BossCell_C|SetShootAtPlayer _array_element_8 false))
                (Utilities|FlowControl|Delay _timebetweenattacks)
                (Variables|Default|SetcanAttack true)))))))
    (:2
      (goto _label))))

(fn ConstructionScript)

(fn BossDeath
  (Audio|PlaySound2D "/Game/SoundEffects/bossdeath.bossdeath" 1.0 1.0 0.0 0 0)
  (Widget|RemovefromParent (Variables|Default|GetBossHealthBar))
  (bind _returnvalue (Actor|GetActorOfClass "/Game/Blueprints/LevelDoor.LevelDoor_C"))
  (Default|OpenDoor _returnvalue))

(fn TakeDamage
  (params (Amount :type Float%20%28double-precision%29))
  (bind _output_get (Variables|Default|SetCurHealth (- (Variables|Default|GetCurHealth) Amount)))
  (Audio|PlaySound2D "/Game/SoundEffects/dooropentest3.dooropentest3" 1.0 1.0 0.0 0 0)
  (if (<= _output_get 0.0)
    (CallFunction|BossDeath)
    (elif (and (<= (Variables|Default|GetCurHealth) (/ (Variables|Default|GetMaxHealth) 2.0)) (< (Variables|Default|GetStage) 2))
      (Audio|PlaySound2D "/Game/SoundEffects/bossstageprogress.bossstageprogress" 1.0 1.0 0.0 0 0)
      (Variables|Default|SetStage 2)
      (Variables|Default|SetAttackTime 0.75))))