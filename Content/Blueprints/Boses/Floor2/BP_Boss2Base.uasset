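; BP_Boss2Base is a base Blueprint for Floor 2 bosses that manages their health.
; TakeDamage lowers CurrentHealth, plays a 2D sound, and at zero or below clamps it to zero and calls BossDeath.
; HealDamage raises health up to MaxHealth and plays a sound.
; BossDeath is an empty function here, and the event graph has no logic.
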(event EventBeginPlay)

(event Collision|EventActorBeginOverlap
  (params (OtherActor :type Actor%20Object%20Reference)))

(event EventTick
  (params (DeltaSeconds :type Float%20%28single-precision%29)))

(fn ConstructionScript)

(fn BossDeath)

(fn TakeDamage
  (params (Amount :type Float%20%28double-precision%29))
  (bind _output_get (Variables|Default|SetCurrentHealth (- (Variables|Default|GetCurrentHealth) Amount)))
  (Audio|PlaySound2D 0 1.0 1.0 0.0 0 0)
  (if (<= _output_get 0.0)
    (Variables|Default|SetCurrentHealth 0.0)
    (CallFunction|BossDeath)))

(fn HealDamage
  (params (Amount :type Float%20%28double-precision%29))
  (bind _maxhealth (Variables|Default|GetMaxHealth))
  (bind _output_get (Variables|Default|SetCurrentHealth (+ (Variables|Default|GetCurrentHealth) Amount)))
  (if (>= _output_get _maxhealth)
    (Variables|Default|SetCurrentHealth _maxhealth))
  (Audio|PlaySound2D 0 1.0 1.0 0.0 0 0))