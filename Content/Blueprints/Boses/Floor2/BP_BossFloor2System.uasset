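; BP_BossFloor2System manages the second-floor dual boss fight against Acamus and Diophomus.
; On BeginPlay it finds both bosses, copies their max health and adds a shared boss health bar widget to the viewport.
; Separate damage functions lower each boss's tracked health and flag its death.
; Once both are dead, it plays a sound, removes the widget and opens the LevelDoor.
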(event EventBeginPlay
  (bind _returnvalue (Actor|GetActorOfClass "/Game/Blueprints/Boses/Floor2/BP_BossFloor2_Acamus.BP_BossFloor2_Acamus_C"))
  (bind _output_get (Variables|Default|SetAcamus _returnvalue))
  (Variables|Default|SetMaxHealth1 (Variables|/Game/Blueprints/Boses/BP_BossDamagableBase.BP_BossDamagableBase_C|GetMaxHealth _output_get))
  (Variables|Default|SetCurHealth1 (Variables|/Game/Blueprints/Boses/BP_BossDamagableBase.BP_BossDamagableBase_C|GetMaxHealth _output_get))
  (bind _returnvalue_2 (Actor|GetActorOfClass "/Game/Blueprints/Boses/Floor2/BP_BossFloor2_Diophomus.BP_BossFloor2_Diophomus_C"))
  (bind _output_get_2 (Variables|Default|SetDiophomus _returnvalue_2))
  (Variables|Default|SetMaxHealth2 (Variables|/Game/Blueprints/Boses/BP_BossDamagableBase.BP_BossDamagableBase_C|GetMaxHealth _output_get_2))
  (Variables|Default|SetCurHealth2 (Variables|/Game/Blueprints/Boses/BP_BossDamagableBase.BP_BossDamagableBase_C|GetMaxHealth _output_get_2))
  (bind _returnvalue_3 (UserInterface|CreateWidget "/Game/UI/UI_BossFloor2HealthBar.UI_BossFloor2HealthBar_C"))
  (bind _output_get_3 (Variables|Default|SetSecondFloorUI _returnvalue_3))
  (UserInterface|Viewport|AddtoViewport _output_get_3 0))

(event Collision|EventActorBeginOverlap
  (params (OtherActor :type Actor%20Object%20Reference)))

(event EventTick
  (params (DeltaSeconds :type Float%20%28single-precision%29)))

(fn ConstructionScript
  (|CallParentFunction))

(fn BossDeath
  (Audio|PlaySound2D 0 1.0 1.0 0.0 0 0)
  (Widget|RemovefromParent (Variables|Default|GetSecondFloorUI))
  (bind _returnvalue (Actor|GetActorOfClass "/Game/Blueprints/LevelDoor.LevelDoor_C"))
  (Default|OpenDoor _returnvalue))

(fn TakeDamage1
  (params (Damage :type Float%20%28double-precision%29))
  (bind _output_get (Variables|Default|SetCurHealth1 (- (Variables|Default|GetCurHealth1) Damage)))
  (if (<= _output_get 0.0)
    (bind _output_get_2 (Variables|Default|SetBoss1Dead true))
    (if (and _output_get_2 (Variables|Default|GetBoss2Dead))
      (CallFunction|BossDeath))))

(fn TakeDamage2
  (params (Damage :type Float%20%28double-precision%29))
  (bind _output_get (Variables|Default|SetCurHealth2 (- (Variables|Default|GetCurHealth2) Damage)))
  (if (<= _output_get 0.0)
    (bind _output_get_2 (Variables|Default|SetBoss2Dead true))
    (if (and _output_get_2 (Variables|Default|GetBoss1Dead))
      (CallFunction|BossDeath))))