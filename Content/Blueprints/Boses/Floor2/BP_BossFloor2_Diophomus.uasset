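; Floor 2 boss Diophomus, a ranged enemy that forwards damage it takes to the BP_BossFloor2System found at BeginPlay.
; While active, a Tick-driven stage machine waits through start-up, then repeatedly picks a random normal, arc or rapid shot after a delay.
; During timed attacks it turns toward the player, spawns turret bullets and pushes itself away when the player is too close.
; Death deactivates it and triggers a blood effect.
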(event EventBeginPlay
  (|CallParentFunction)
  (bind _returnvalue (Actor|GetActorOfClass "/Game/Blueprints/Boses/Floor2/BP_BossFloor2System.BP_BossFloor2System_C"))
  (Variables|Default|SetBoss _returnvalue))

(event Collision|EventActorBeginOverlap
  (params (OtherActor :type Actor%20Object%20Reference))
  (|CallParentFunction OtherActor) ; This node is disabled and will not be called.\nDrag off pins to build functionality.
)

(event EventTick
  (params (DeltaSeconds :type Float%20%28single-precision%29))
  (bind _returnvalue (Game|Player|GetPlayerPawn 0))
  (bind _returnvalue_2 (Transformation|GetActorLocation))
  (bind _distancefrompayer (Variables|Default|GetDistanceFromPayer))
  (bind _returnvalue_3 (Transformation|GetActorLocation _returnvalue))
  (bind _returnvalue_4 (- _returnvalue_2 _returnvalue_3))
  (bind (_x _y) (Math|Vector|BreakVector _returnvalue_4))
  (|CallParentFunction DeltaSeconds)
  (if (Variables|Default|GetisActive)
    (switch int (Variables|Default|GetStage)
      (:0
        (bind _output_get (Variables|Default|Settimer (+ (Variables|Default|Gettimer) DeltaSeconds)))
        (if (>= _output_get (Variables|Default|GetStartUpTime))
          (Variables|Default|Settimer 0.0)
          (Variables|Default|SetStage 1)))
      (:1
        (if (not (Variables|Default|GetinAction))
          (Utilities|FlowControl|Delay (Variables|Default|GetTimeBetweenAttacks))
          (Variables|Default|SetinAction true)
          (switch int (Math|Random|RandomIntegerinRange 0 2)
            (:Default
              (Variables|Default|SetnormalShoot true :!label _label))
            (:0
              (goto _label))
            (:1
              (Variables|Default|SetarcShoot true))
            (:2
              (Variables|Default|SetrapidShoot true)))
          (else
            (bind _output_get_2 (Variables|Default|SetattackTimer (+ DeltaSeconds (Variables|Default|GetattackTimer))))
            (if (>= _output_get_2 (Variables|Default|GetAttackTime))
              (Variables|Default|SetattackTimer 0.0)
              (Variables|Default|SetinAction false)
              (Variables|Default|SetnormalShoot false)
              (Variables|Default|SetarcShoot false)
              (Variables|Default|SetrapidShoot false)
              (else
                (if (< (Math|Vector|Distance(Vector) _returnvalue_3 _returnvalue_2) _distancefrompayer)
                  (Physics|AddForce (Variables|Character|GetCharacterMovement) (* (Math|Vector|MakeVector _x _y 0.0) (* _distancefrompayer 5.0))))
                (if (Variables|Default|GetnormalShoot)
                  (Transformation|AddActorLocalRotation (Math|Rotator|FindRelativeLookatRotation (Transformation|GetActorTransform) (Transformation|GetActorLocation (Game|GetPlayerCharacter 0))) false false)
                  (bind _output_get_3 (Variables|Default|Settimer (+ (Variables|Default|Gettimer) DeltaSeconds)))
                  (if (>= _output_get_3 (Variables|Default|GetTimeBetweenBullets))
                    (Variables|Default|Settimer 0.0)
                    (Audio|PlaySound2D "/Game/SoundEffects/turretshoot.turretshoot" 1.0 1.0 0.0 0 0)
                    (Game|SpawnActorfromClass "/Game/Blueprints/TurretBullet.TurretBullet_C" (Transformation|GetWorldTransform (Variables|Default|GetBulletSpawnPoint)) "AlwaysSpawn" "MultiplyWithRoot" 0 0))
                  (elif (Variables|Default|GetarcShoot)
                    (Transformation|AddActorLocalRotation (Math|Rotator|FindRelativeLookatRotation (Transformation|GetActorTransform) (Transformation|GetActorLocation (Game|GetPlayerCharacter 0))) false false)
                    (bind _output_get_4 (Variables|Default|Settimer (+ (Variables|Default|Gettimer) DeltaSeconds)))
                    (if (>= _output_get_4 (Variables|Default|GetTimeBetweenBullets))
                      (Variables|Default|Settimer 0.0)
                      (for _index (range 0 (Variables|Default|GetArcShotBulletCount))
                        (Transformation|AddActorLocalRotation "0.000000,10.000000,0.000000" false false)
                        (Audio|PlaySound2D "/Game/SoundEffects/turretshoot.turretshoot" 1.0 1.0 0.0 0 0)
                        (Game|SpawnActorfromClass "/Game/Blueprints/TurretBullet.TurretBullet_C" (Transformation|GetWorldTransform (Variables|Default|GetBulletSpawnPoint)) "AlwaysSpawn" "MultiplyWithRoot" 0 0)))
                    (elif (Variables|Default|GetrapidShoot)
                      (Transformation|AddActorLocalRotation (Math|Rotator|FindRelativeLookatRotation (Transformation|GetActorTransform) (Transformation|GetActorLocation (Game|GetPlayerCharacter 0))) false false)
                      (bind _output_get_5 (Variables|Default|Settimer (+ (Variables|Default|Gettimer) DeltaSeconds)))
                      (if (>= _output_get_5 (/ (Variables|Default|GetTimeBetweenBullets) 2.0))
                        (Variables|Default|Settimer 0.0)
                        (Audio|PlaySound2D "/Game/SoundEffects/turretshoot.turretshoot" 1.0 1.0 0.0 0 0)
                        (Game|SpawnActorfromClass "/Game/Blueprints/TurretBullet.TurretBullet_C" (Transformation|GetWorldTransform (Variables|Default|GetBulletSpawnPoint)) "AlwaysSpawn" "MultiplyWithRoot" 0 0)))))))))))))

(fn ConstructionScript
  (|CallParentFunction))

(fn TakeDamage
  (params (Amount :type Float%20%28double-precision%29))
  (|CallParentFunction Amount)
  (Default|TakeDamage2 (Variables|Default|GetBoss) Amount))

(fn Die
  (|CallParentFunction)
  (Variables|Default|SetisActive false)
  (Components|Activation|Activate (Variables|Default|GetBoss2Blood) false))