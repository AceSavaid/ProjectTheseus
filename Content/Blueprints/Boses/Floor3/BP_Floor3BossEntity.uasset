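; Floor 3 boss entity that fires radial bullet bursts and forwards the damage it takes to the shared BP_Floor3BossSystem found at BeginPlay.
; Tick runs a staged timer: a start-up delay, then repeated attacks separated by a cooldown.
; Each attack spawns TurretBullets evenly spaced around the actor by yaw.
; The random attack selector has only this one pattern, and an AttackTimer loop for sustained fire is left unconnected.
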(event EventBeginPlay
  (|CallParentFunction)
  (Variables|Default|SetCurrentHealth (Variables|Default|GetMaxHealth))
  (bind _returnvalue (Actor|GetActorOfClass "/Game/Blueprints/Boses/Floor3/BP_Floor3BossSystem.BP_Floor3BossSystem_C"))
  (Variables|Default|SetBoss _returnvalue))

(event Collision|EventActorBeginOverlap
  (params (OtherActor :type Actor%20Object%20Reference))
  (|CallParentFunction OtherActor) ; This node is disabled and will not be called.\nDrag off pins to build functionality.
)

(event EventTick
  (params (DeltaSeconds :type Float%20%28single-precision%29))
  (bind _bulletspershot (Variables|Default|GetBulletsPerShot))
  (|CallParentFunction DeltaSeconds)
  (switch int (Variables|Default|GetStage)
    (:Default
      (switch int (Math|Random|RandomIntegerinRange 0 0) :!label _label
        (:0
          (for _index (range 0 (- _bulletspershot 1))
            (Game|SpawnActorfromClass "/Game/Blueprints/TurretBullet.TurretBullet_C" (Math|Transform|MakeTransform (Transformation|GetActorLocation) (Math|Rotator|MakeRotator 0.0 0.0 (Math|Conversions|ToFloat(Integer) (* _index (/ 360 _bulletspershot))))) "AlwaysSpawn" "MultiplyWithRoot" 0 0))
          (Variables|Default|SetdidAction true))))
    (:0
      (bind _output_get (Variables|Default|Settimer (+ (Variables|Default|Gettimer) DeltaSeconds)))
      (if (>= _output_get (Variables|Default|GetStartUpTime))
        (Variables|Default|Settimer 0.0)
        (Variables|Default|SetStage 1)))
    (:1
      (if (not (Variables|Default|GetdidAction))
        (goto _label)
        (else
          (bind _output_get_2 (Variables|Default|Settimer (+ DeltaSeconds (Variables|Default|Gettimer))))
          (if (>= _output_get_2 (Variables|Default|GetTimeBetweenAttacks))
            (Variables|Default|Settimer 0.0)
            (Variables|Default|SetdidAction false)))))))

(fn ConstructionScript
  (|CallParentFunction))

(fn TakeDamage
  (params (Amount :type Float%20%28double-precision%29))
  (|CallParentFunction Amount)
  (Default|TakeDamage (Variables|Default|GetBoss) Amount))

(fn Die
  (|CallParentFunction))