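; BP_Floor3BossSystem is the manager for the Floor 3 boss fight, tracking boss health, stage and death.
; On BeginPlay it fills health, shows the health bar widget and caches the BP_Floor3BossEntity actor.
; TakeDamage subtracts health and advances Stage at half and quarter health with sound cues, at most one stage per hit.
; At zero health, BossDeath plays a sound, removes the bar and opens the LevelDoor.
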(event EventBeginPlay
  (|CallParentFunction)
  (Variables|Default|SetCurHealth (Variables|Default|GetMaxHealth))
  (bind _returnvalue (UserInterface|CreateWidget "/Game/UI/UI_BossFloor3HealthBar.UI_BossFloor3HealthBar_C"))
  (bind _output_get (Variables|Default|SetBossUI _returnvalue))
  (UserInterface|Viewport|AddtoViewport _output_get 0)
  (bind _returnvalue_2 (Actor|GetActorOfClass "/Game/Blueprints/Boses/Floor3/BP_Floor3BossEntity.BP_Floor3BossEntity_C"))
  (Variables|Default|SetBossEntity _returnvalue_2))

(event Collision|EventActorBeginOverlap
  (params (OtherActor :type Actor%20Object%20Reference))
  (|CallParentFunction OtherActor) ; This node is disabled and will not be called.\nDrag off pins to build functionality.
)

(event EventTick
  (params (DeltaSeconds :type Float%20%28single-precision%29))
  (|CallParentFunction DeltaSeconds) ; This node is disabled and will not be called.\nDrag off pins to build functionality.
)

(fn ConstructionScript
  (|CallParentFunction))

(fn TakeDamage
  (params (Amount :type Float%20%28double-precision%29))
  (bind _output_get (Variables|Default|SetCurHealth (- (Variables|Default|GetCurHealth) Amount)))
  (Audio|PlaySound2D 0 1.0 1.0 0.0 0 0)
  (if (<= _output_get 0.0)
    (CallFunction|BossDeath)
    (elif (and (<= (Variables|Default|GetCurHealth) (/ (Variables|Default|GetMaxHealth) 2.0)) (<= (Variables|Default|GetStage) 1))
      (Audio|PlaySound2D 0 1.0 1.0 0.0 0 0)
      (Variables|Default|SetStage 2)
      (elif (and (<= (Variables|Default|GetCurHealth) (/ (Variables|Default|GetMaxHealth) 4.0)) (<= (Variables|Default|GetStage) 2))
        (Audio|PlaySound2D 0 1.0 1.0 0.0 0 0)
        (Variables|Default|SetStage 3)))))

(fn BossDeath
  (Audio|PlaySound2D 0 1.0 1.0 0.0 0 0)
  (Widget|RemovefromParent (Variables|Default|GetBossUI))
  (bind _returnvalue (Actor|GetActorOfClass "/Game/Blueprints/LevelDoor.LevelDoor_C"))
  (Default|OpenDoor _returnvalue))