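; Boss2Bullet is a projectile actor that damages the player on contact.
; Each tick it moves along its Arrow's forward vector without sweeping, scaled by Speed, and destroys itself once its timer reaches LiveTime.
; Sphere overlap with BP_Player applies Damage and destroys the bullet, opening the DeathScreen level if TakeDamage returns true.
; Overlap with a BasicEnemy destroys the bullet without dealing damage.
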(event OnComponentBeginOverlap(SphereCollider)
  (params (OverlappedComponent :type Primitive%20Component%20Object%20Reference) (OtherActor :type Actor%20Object%20Reference) (OtherComp :type Primitive%20Component%20Object%20Reference) (OtherBodyIndex :type Integer) (bFromSweep :type Boolean) (SweepResult :type Hit%20Result%20Structure%20%28by%20ref%29))
  (bind _asbp_player (Utilities|Casting|CastToBP_Player OtherActor)
    (:then
      (bind _diedfromdamage (Default|TakeDamage _asbp_player (Variables|Default|GetDamage)))
      (Actor|DestroyActor)
      (if _diedfromdamage
        (Game|OpenLevel(byName) "DeathScreen")))
    (:CastFailed
      (Utilities|Casting|CastToBasicEnemy OtherActor)
      (Actor|DestroyActor))))

(event EventTick
  (params (DeltaSeconds :type Float%20%28single-precision%29))
  (bind _defaultsceneroot (Variables|Default|GetDefaultSceneRoot))
  (Transformation|SetWorldLocation _defaultsceneroot (+ (Transformation|GetWorldLocation _defaultsceneroot) (* (Math|Vector|GetForwardVector (Variables|Default|GetArrow)) (* (* DeltaSeconds (Variables|Default|GetSpeed)) 1e+02))) false false)
  (bind _output_get (Variables|Default|Settimer (+ DeltaSeconds (Variables|Default|Gettimer))))
  (if (>= _output_get (Variables|Default|GetLiveTime))
    (Actor|DestroyActor)))

(fn ConstructionScript)