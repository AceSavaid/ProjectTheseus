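; Basic enemy that chases the player with AIMoveTo, tuned by a single EnemyAggression value.
; Aggression scales walk speed and inversely scales both the start delay and the pause before re-chasing after each successful move.
; A failed move only prints its result, ending the chase loop.
; Tick turns the text render toward the player camera, and overlaps print the other actor's name for debugging.
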(event EventBeginPlay
  (Variables|/Script/Engine.CharacterMovementComponent|SetMaxWalkSpeed (Variables|Character|GetCharacterMovement) (* (Variables|Default|GetEnemyAggression) 1e+02))
  (Utilities|FlowControl|Delay (Math|Float|Power (Variables|Default|GetEnemyAggression) -1.0))
  (bind _asbp_player (Utilities|Casting|CastToBP_Player (Game|GetPlayerCharacter 0)))
  (bind _movementresult (AI|AIMoveTo (Pawn|GetControlledPawn (AI|GetAIController self)) "0, 0, 0" _asbp_player 5.0 false :!label _label)
    (:then
      _)
    (:OnSuccess
      (Utilities|FlowControl|Delay (* (Math|Float|Power (Variables|Default|GetEnemyAggression) -1.0) 5.0))
      (goto _label))
    (:OnFail
      _))
  (Development|PrintString (Utilities|String|EnumtoString _movementresult)))

(event EventTick
  (params (DeltaSeconds :type Float%20%28single-precision%29))
  (bind _asbp_player (Utilities|Casting|CastToBP_Player (Game|GetPlayerCharacter 0)))
  (Transformation|SetWorldRotation (Variables|Default|GetTextRender) (Math|Rotator|MakeRotator (.roll (Transformation|GetWorldRotation (Variables|/Game/Blueprints/BP_Player.BP_Player_C|GetCamera _asbp_player))) (.pitch (Transformation|GetWorldRotation (Variables|/Game/Blueprints/BP_Player.BP_Player_C|GetCamera _asbp_player))) (- (.yaw (Transformation|GetWorldRotation (Variables|/Game/Blueprints/BP_Player.BP_Player_C|GetCamera _asbp_player))) 1.8e+02)) false false))

(event Collision|EventActorBeginOverlap
  (params (OtherActor :type Actor%20Object%20Reference))
  (Development|PrintString (Utilities|GetDisplayName OtherActor)))

(fn ConstructionScript)