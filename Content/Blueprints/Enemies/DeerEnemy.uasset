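; DeerEnemy is a hostile deer character that chases the player and deals damage in melee, opening the DeathScreen level when TakeDamage returns true.
; An aggression value drives walk speed, animation play rate and the delays between actions.
; BeginPlay starts a looping AI MoveTo chase that plays an attack animation on arrival and hits only within close range.
; A material swap on its static mesh marks each non-lethal hit until the chase resumes.
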(event EventBeginPlay
  (bind _mesh (Variables|Character|GetMesh))
  (bind _staticmesh (Variables|Default|GetStaticMesh))
  (bind _mesh_2 (Variables|Character|GetMesh))
  (Variables|/Script/Engine.CharacterMovementComponent|SetMaxWalkSpeed (Variables|Character|GetCharacterMovement) (* (Variables|Default|GetEnemyAggression) 1e+02))
  (Utilities|FlowControl|Delay (Math|Float|Power (Variables|Default|GetEnemyAggression) -1.0))
  (bind _asbp_player (Utilities|Casting|CastToBP_Player (Game|GetPlayerCharacter 0)))
  (Components|Animation|PlayAnimation _mesh "/Game/AnimationStuff/Wolf/WolfDeer_WalkAnim.WolfDeer_WalkAnim" true :!label _label)
  (Components|Timeline|SetPlayRate _mesh (/ (Variables|Default|GetEnemyAggression) 4.0))
  (AI|AIMoveTo (Pawn|GetControlledPawn (AI|GetAIController self)) "0, 0, 0" _asbp_player 5.0 false
    (:OnSuccess
      (bind _asbp_player_2 (Utilities|Casting|CastToBP_Player _asbp_player))
      (Components|Animation|PlayAnimation _mesh_2 "/Game/AnimationStuff/Wolf/WolfDeer_AttackAnim.WolfDeer_AttackAnim" true)
      (Components|Timeline|SetPlayRate _mesh_2 (/ (Variables|Default|GetEnemyAggression) 4.0))
      (if (> (Transformation|GetDistanceTo _asbp_player_2) 1.5e+02)
        (Utilities|FlowControl|Delay (* (Math|Float|Power (Variables|Default|GetEnemyAggression) -1.0) 5.0) :!label _label_2)
        (Rendering|Material|SetMaterial _staticmesh 0 "/Engine/EngineMaterials/WorldGridMaterial.WorldGridMaterial")
        (goto _label)
        (else
          (bind _diedfromdamage (Default|TakeDamage _asbp_player_2 (Variables|Default|GetEnemyDamage)))
          (Audio|PlaySound2D "/Game/SoundEffects/playerhurt.playerhurt" 1.0 1.0 0.0 0 0)
          (if _diedfromdamage
            (Game|OpenLevel(byName) "DeathScreen")
            (else
              (Rendering|Material|SetMaterial _staticmesh 0 "/Engine/MapTemplates/Sky/M_Procedural_Sky_Night.M_Procedural_Sky_Night")
              (goto _label_2))))))))

(event Collision|EventActorBeginOverlap
  (params (OtherActor :type Actor%20Object%20Reference)))

(event EventTick
  (params (DeltaSeconds :type Float%20%28single-precision%29)))

(fn ConstructionScript)