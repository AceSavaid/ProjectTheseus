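; Slime enemy that chases the player and deals melee damage, with EnemyAggression scaling walk speed, animation rate and delays.
; From BeginPlay it loops through AI MoveTo, attack animation, range check and an inversely scaled cooldown.
; A close hit calls TakeDamage on BP_Player and plays a hurt sound, then either opens DeathScreen or swaps the sphere materials until the cooldown ends.
; Only MoveTo's success branch continues the loop.
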(event EventBeginPlay
  (bind _mesh (Variables|Character|GetMesh))
  (bind _mesh_2 (Variables|Character|GetMesh))
  (Variables|/Script/Engine.CharacterMovementComponent|SetMaxWalkSpeed (Variables|Character|GetCharacterMovement) (* (Variables|Default|GetEnemyAggression) 1e+02))
  (Utilities|FlowControl|Delay (Math|Float|Power (Variables|Default|GetEnemyAggression) -1.0))
  (bind _asbp_player (Utilities|Casting|CastToBP_Player (Game|GetPlayerCharacter 0)))
  (Components|Animation|PlayAnimation _mesh_2 "/Game/AnimationStuff/Slime/Slime_MoveAnim.Slime_MoveAnim" true :!label _label)
  (Components|Timeline|SetPlayRate _mesh_2 (/ (Variables|Default|GetEnemyAggression) 4.0))
  (AI|AIMoveTo (Pawn|GetControlledPawn (AI|GetAIController self)) "0, 0, 0" _asbp_player 5.0 false
    (:OnSuccess
      (Components|Animation|PlayAnimation _mesh "/Game/AnimationStuff/Slime/Slime_AttackAnim.Slime_AttackAnim" true)
      (Components|Timeline|SetPlayRate _mesh (/ (Variables|Default|GetEnemyAggression) 4.0))
      (if (> (Transformation|GetDistanceTo _asbp_player) 1.5e+02)
        (Utilities|FlowControl|Delay (* (Math|Float|Power (Variables|Default|GetEnemyAggression) -1.0) 5.0) :!label _label_2)
        (Rendering|Material|SetMaterial (Variables|Default|GetSphere1) 0 "/Engine/MapTemplates/Materials/BasicAsset03.BasicAsset03")
        (goto _label)
        (else
          (bind _diedfromdamage (Default|TakeDamage _asbp_player (Variables|Default|GetEnemyDamage)))
          (Audio|PlaySound2D "/Game/SoundEffects/playerhurt.playerhurt" 1.0 1.0 0.0 0 0)
          (if _diedfromdamage
            (Game|OpenLevel(byName) "DeathScreen")
            (else
              (Rendering|Material|SetMaterial (Variables|Default|GetSphere1) 0 "/Engine/MapTemplates/Sky/M_Procedural_Sky_Morning.M_Procedural_Sky_Morning")
              (goto _label_2))))))))

(fn ConstructionScript)