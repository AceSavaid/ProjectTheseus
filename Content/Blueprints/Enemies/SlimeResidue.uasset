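; SlimeResidue is an enemy slime hazard that damages the player standing in it and destroys itself after a fixed delay.
; Player overlap restarts a Timeline whose every update applies slime damage; leaving the overlap stops it.
; When the player's damage call returns true, the game instance transitions to the death screen level.
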(event EventBeginPlay
  (Utilities|FlowControl|Delay 1e+01)
  (Actor|DestroyActor))

(event Collision|EventActorBeginOverlap
  (params (OtherActor :type Actor%20Object%20Reference))
  (bind _asbp_player (Utilities|Casting|CastToBP_Player OtherActor))
  (Timeline|Timeline PlayFromStart
    (:Update
      (bind _diedfromdamage (Default|TakeDamage _asbp_player (Variables|Default|GetSlimeDamage)))
      (if _diedfromdamage
        (Default|TransitiontoLevel (Default|GetGameInstance _asbp_player) "DeathScreen" _asbp_player)))))

(event Collision|EventActorEndOverlap
  (params (OtherActor :type Actor%20Object%20Reference))
  (Utilities|Casting|CastToBP_Player OtherActor)
  (Timeline|Timeline Stop
    (:Update
      (bind _diedfromdamage (Default|TakeDamage (stale Collision|EventActorBeginOverlap _asbp_player) (Variables|Default|GetSlimeDamage)))
      (if _diedfromdamage
        (Default|TransitiontoLevel (Default|GetGameInstance (stale Collision|EventActorBeginOverlap _asbp_player)) "DeathScreen" (stale Collision|EventActorBeginOverlap _asbp_player))))))

(fn ConstructionScript)