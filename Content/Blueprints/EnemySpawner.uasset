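; Enemy spawner actor that spawns random deer and slime enemies at its own X/Y and a fixed height.
; Tick increments the player's CurrentEnemies while below MaxEnemies, before a Delay gates the spawn, so increments can outpace spawns.
; The GameInstance's CompletedLevels selects one of three enemy pools, shifting to later variants as levels accumulate.
; Some spawn nodes in the later pools have no class assigned.
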(event EventBeginPlay
  (bind _returnvalue (Transformation|GetActorLocation))
  (Variables|Default|SetSpawnTransform (Math|Transform|MakeTransform (Math|Vector|MakeVector (.x _returnvalue) (.y _returnvalue) -9e+01) (Transformation|GetActorRotation))))

(event Collision|EventActorBeginOverlap
  (params (OtherActor :type Actor%20Object%20Reference)))

(event EventTick
  (params (DeltaSeconds :type Float%20%28single-precision%29))
  (bind _asbp_player (Utilities|Casting|CastToBP_Player (Game|GetPlayerCharacter 0)))
  (if (< (Variables|/Game/Blueprints/BP_Player.BP_Player_C|GetCurrentEnemies _asbp_player) (Variables|/Game/Blueprints/BP_Player.BP_Player_C|GetMaxEnemies _asbp_player))
    (Math|Integer|IncrementInt (Variables|/Game/Blueprints/BP_Player.BP_Player_C|GetCurrentEnemies _asbp_player)
      (:%20%20
        (Utilities|FlowControl|Delay 2.0)
        (if (<= (Variables|/Game/Blueprints/Persistence/GI_Persistent.GI_Persistent_C|GetCompletedLevels (Default|GetGameInstance _asbp_player)) 10)
          (if (== (Math|Integer|%(Integer) (Math|Random|RandomIntegerinRange 1 2) 2) 0)
            (Game|SpawnActorfromClass "/Game/Blueprints/Enemies/DeerEnemy.DeerEnemy_C" (Variables|Default|GetSpawnTransform) "AlwaysSpawn" "MultiplyWithRoot" 0 0 :!label _label)
            (else
              (Game|SpawnActorfromClass "/Game/Blueprints/Enemies/SlimeEnemy2.SlimeEnemy2_C" (Variables|Default|GetSpawnTransform) "AlwaysSpawn" "MultiplyWithRoot" 0 0 :!label _label_2)))
          (elif (<= (Variables|/Game/Blueprints/Persistence/GI_Persistent.GI_Persistent_C|GetCompletedLevels (Default|GetGameInstance _asbp_player)) 20)
            (switch int (Math|Random|RandomIntegerinRange 0 3)
              (:0
                (goto _label))
              (:1
                (goto _label_2))
              (:2
                (Game|SpawnActorfromClass "/Game/Blueprints/Enemies/DeerEnemy2.DeerEnemy2_C" (Variables|Default|GetSpawnTransform) "Undefined" "MultiplyWithRoot" 0 0 :!label _label_3))
              (:3
                (Game|SpawnActorfromClass "/Game/Blueprints/Enemies/Slime3.Slime3_C" (Variables|Default|GetSpawnTransform) "Undefined" "MultiplyWithRoot" 0 0 :!label _label_4)))
            (else
              (switch int (Math|Random|RandomIntegerinRange 0 3)
                (:0
                  (goto _label_3))
                (:1
                  (Game|SpawnActorfromClass "/Game/Blueprints/Enemies/DeerEnemy3.DeerEnemy3_C" (Variables|Default|GetSpawnTransform) "Undefined" "MultiplyWithRoot" 0 0))
                (:2
                  (goto _label_4))
                (:3
                  (Game|SpawnActorfromClass "/Game/Blueprints/Enemies/Slime4.Slime4_C" (Variables|Default|GetSpawnTransform) "Undefined" "MultiplyWithRoot" 0 0))))))))))

(fn ConstructionScript)