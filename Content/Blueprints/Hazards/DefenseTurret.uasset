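; DefenseTurret is a hazard Blueprint that spins its cube and fires TurretBullet actors at a timed interval.
; Every Tick adds a fixed local rotation to the cube, independent of frame time, and spawns a bullet at the arrow's world transform when shooting is allowed.
; A delta-time accumulator gates the next shot, playing the shoot sound and firing as soon as the interval elapses, with no targeting logic.
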(event EventTick
  (params (DeltaSeconds :type Float%20%28single-precision%29))
  (Transformation|AddLocalRotation (Variables|Default|GetCube) (Variables|Default|GetRotateAngle) false false)
  (if (Variables|Default|GetCanshoot)
    (Game|SpawnActorfromClass "/Game/Blueprints/TurretBullet.TurretBullet_C" (Transformation|GetWorldTransform (Variables|Default|GetArrow)) "AlwaysSpawn" "MultiplyWithRoot" 0 0 :!label _label)
    (Variables|Default|SetCanshoot false)
    (else
      (bind _output_get (Variables|Default|SetBullet%20timer (+ DeltaSeconds (Variables|Default|GetBullet%20timer))))
      (if (>= _output_get (Variables|Default|GetTimeBetweenshots))
        (Variables|Default|SetBullet%20timer 0.0)
        (Variables|Default|SetCanshoot true)
        (Audio|SpawnSoundatLocation "/Game/SoundEffects/turretshoot.turretshoot" (Transformation|GetActorLocation) "0, 0, 0" 1.0 1.0 0.0 0 0)
        (goto _label)))))

(fn ConstructionScript)