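; WallLaser is a hazard Blueprint that fires a laser in timed on/off cycles.
; Tick accumulates delta time in a shared timer to alternate between firing and resting phases, playing a 2D sound at each switch.
; While firing, a second timer repeatedly spawns LazerBeam actors at the Arrow component's world transform, so the laser is a stream of spawned actors.
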(event EventTick
  (params (DeltaSeconds :type Float%20%28single-precision%29))
  (if (Variables|Default|GetCanshoot)
    (bind _output_get (Variables|Default|Settimer (+ DeltaSeconds (Variables|Default|Gettimer))))
    (if (>= _output_get (Variables|Default|GetLazerDuration))
      (Variables|Default|SetCanShoot false)
      (Variables|Default|Settimer 0.0)
      (Audio|PlaySound2D "/Game/SoundEffects/lazerwinddown.lazerwinddown" 1.0 1.0 0.0 0 0)
      (else
        (bind _output_get_2 (Variables|Default|Settimer2 (+ (Variables|Default|Gettimer2) DeltaSeconds)))
        (if (>= _output_get_2 (Variables|Default|GetShootDely))
          (Variables|Default|Settimer2 0.0)
          (Game|SpawnActorfromClass "/Game/Blueprints/LazerBeam.LazerBeam_C" (Transformation|GetWorldTransform (Variables|Default|GetArrow)) "AlwaysSpawn" "MultiplyWithRoot" 0 0))))
    (else
      (bind _output_get_3 (Variables|Default|Settimer (+ DeltaSeconds (Variables|Default|Gettimer))))
      (if (>= _output_get_3 (Variables|Default|GetTimeBetweenshots))
        (Variables|Default|Settimer 0.0)
        (Variables|Default|SetCanshoot true)
        (Audio|PlaySound2D "/Game/SoundEffects/dooropentest2.dooropentest2" 1.0 1.0 0.0 0 0)))))

(fn ConstructionScript)