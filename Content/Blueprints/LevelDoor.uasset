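; LevelDoor is a door actor that rises vertically when its OpenDoor event is called.
; OpenDoor plays a sound at the door and runs the DoorOpening timeline, moving the root upward with sweep.
; Each update lerps from the current height toward a fixed offset above it, so movement accumulates.
; Opened blocks reopening but is set only when the timeline finishes, so calls during opening repeat the sound.
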(event Custom|OpenDoor
  (bind _defaultsceneroot (Variables|Default|GetDefaultSceneRoot))
  (bind _returnvalue (Transformation|GetWorldLocation _defaultsceneroot))
  (if (not (Variables|Default|GetOpened))
    (Audio|SpawnSoundatLocation "/Game/SoundEffects/dooropentest.dooropentest" (Transformation|GetActorLocation) "0, 0, 0" 1.0 1.0 0.0 0 0)
    (bind _dooropening (Timeline|DoorOpening Play)
      (:Update
        (Transformation|SetWorldLocation _defaultsceneroot (Math|Vector|MakeVector (.x _returnvalue) (.y _returnvalue) (Math|Float|Lerp (.z _returnvalue) (+ (.z _returnvalue) 3e+01) _dooropening)) true false))
      (:Finished
        (Variables|Default|SetOpened true)))))

(event Collision|EventActorBeginOverlap
  (params (OtherActor :type Actor%20Object%20Reference)))

(event EventTick
  (params (DeltaSeconds :type Float%20%28single-precision%29)))

(fn ConstructionScript)