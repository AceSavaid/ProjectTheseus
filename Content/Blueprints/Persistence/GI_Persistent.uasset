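; GI_Persistent is a game instance that carries player state between room levels.
; On Init it fills a list of level names covering a test level and the first-floor rooms.
; TransitionToLevel copies the player's equips, base health, walk speed and weapon damage into its variables, flags that a transition should load, then opens the named level.
; Restoring that state onto the player is not handled here.
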(event Custom|TransitionToLevel
  (params (Level :type Name) (Player :type BP%20Player%20Object%20Reference))
  (CallFunction|GatherPlayerState Player)
  (Variables|Default|SetShouldLoadTransition true)
  (Game|OpenLevel(byName) Level))

(event EventInit
  (Variables|Default|SetLevels (Utilities|Array|MakeArray "TestLevel" "Floor1Room2" "Floor1Room3" "Floor1Room4" "Floor1Room5" "Floor1Room6" "Floor1Room7" "Floor1Room8" "Floor1Room9" "Floor1Room10" "Floor1Room11" "Floor1Room12" "Floor1Room13" "Floor1Room14")))

(fn GatherPlayerState
  (params (Player :type BP%20Player%20Object%20Reference))
  (Variables|Default|SetEquips (Variables|/Game/Blueprints/BP_Player.BP_Player_C|GetEquips Player))
  (Variables|Default|SetHealth (Variables|/Game/Blueprints/BP_Player.BP_Player_C|GetbaseHealth Player))
  (Variables|Default|SetSpeed (Variables|/Game/Blueprints/BP_Player.BP_Player_C|GetcurrentWalkSpeed Player))
  (Variables|Default|SetDamage (Variables|/Game/Blueprints/BP_Player.BP_Player_C|GetWeaponDamage Player)))