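; BloodLustPickup is a powerup actor that grants the player the BloodLust upgrade, described as healing from killing enemies.
; When BP_Player overlaps it, it enables the BloodLust flag and raises the BloodLust value by a small increment, so repeat pickups stack.
; It then adds a new BP_ListData entry with name, description and icon to the player's upgrade list and destroys itself.
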(event EventBeginPlay)

(event Collision|EventActorBeginOverlap
  (params (OtherActor :type Actor%20Object%20Reference))
  (bind _asbp_player (Utilities|Casting|CastToBP_Player OtherActor))
  (if (Variables|/Game/Blueprints/BP_Player.BP_Player_C|GethasBloodLust _asbp_player)
    _
    (else
      (Variables|/Game/Blueprints/BP_Player.BP_Player_C|SethasBloodLust _asbp_player true)))
  (Variables|/Game/Blueprints/BP_Player.BP_Player_C|SetBloodLustValue _asbp_player (+ (Variables|/Game/Blueprints/BP_Player.BP_Player_C|GetBloodLustValue _asbp_player) 0.02))
  (bind _returnvalue (Game|ConstructObjectfromClass "/Game/UI/UpgradeBackEnd/BP_ListData.BP_ListData_C"))
  (Default|InitiazieData _returnvalue "BloodLust" "Heal from killing enemies" "/Game/StuffThatCouldBeScrap/Cloak.Cloak")
  (Default|AddUpgradetoList _asbp_player _returnvalue)
  (Actor|DestroyActor))

(event EventTick
  (params (DeltaSeconds :type Float%20%28single-precision%29)))

(fn ConstructionScript)