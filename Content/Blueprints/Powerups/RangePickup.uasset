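; Range powerup pickup that extends the player's bullet lifetime by GivenRange on overlap with BP_Player.
; On BeginPlay two timelines animate it, one driving yaw for a spin and one setting absolute world Z for a hover.
; On pickup it also adds a BP_ListData "RangeUp" entry with icon and updated factor to the player's upgrade list, then destroys itself.
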(event EventBeginPlay
  (bind _returnvalue (Transformation|GetActorLocation))
  (bind _returnvalue_2 (Transformation|GetActorRotation))
  (Utilities|FlowControl|Sequence
    (:then_0
      (bind _speener (Timeline|Timeline Play)
        (:Update
          (Transformation|SetActorRotation (Math|Rotator|MakeRotator (.roll _returnvalue_2) (.pitch _returnvalue_2) _speener)))))
    (:then_1
      ;[1 1 1] length of 2pi
      (bind _hooverer (Timeline|Timeline_0 Play)
        (:Update
          (Transformation|SetActorLocation (Math|Vector|MakeVector (.x _returnvalue) (.y _returnvalue) (* _hooverer 2e+01)) false false))))))

(event Collision|EventActorBeginOverlap
  (params (OtherActor :type Actor%20Object%20Reference))
  (bind _asbp_player (Utilities|Casting|CastToBP_Player OtherActor))
  (Variables|/Game/Blueprints/BP_Player.BP_Player_C|SetBulletLifetime _asbp_player (+ (Variables|/Game/Blueprints/BP_Player.BP_Player_C|GetBulletLifetime _asbp_player) (Variables|Default|GetGiven%20Range)))
  (bind _returnvalue (Game|ConstructObjectfromClass "/Game/UI/UpgradeBackEnd/BP_ListData.BP_ListData_C"))
  (Default|InitiazieData _returnvalue "RangeUp" "Increases Range " (- (Variables|/Game/Blueprints/BP_Player.BP_Player_C|GetBulletLifetime _asbp_player) 2.0) "/Game/Textures/UI/Icons/roboarmicon.roboarmicon")
  (Default|AddUpgradetoList _asbp_player _returnvalue)
  (Actor|DestroyActor))

(event EventTick
  (params (DeltaSeconds :type Float%20%28single-precision%29)))

(fn ConstructionScript)